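; Enemy character that constantly walks forward, damages what its attack trace hits, and ragdolls when a Player-tagged actor overlaps its DamageCollision.
; Each tick, floor and wall traces drive a DoOnce into a FlipFlop that stops movement and adds rotation, though both rotations are zero.
; The floor check repeats the attack's sphere trace from AttackDamagePos.
; Death disables movement, ignores Pawn and Camera collision, and stops the damage trace.
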(event `self.ReceiveTick`
  (params (DeltaSeconds :type "Float (single-precision)"))
  (bind _charactermovement (`self.CharacterMovement`))
  (`|ExecutionSequence`
    (:`then_0`
      (bind _floor_detected_ (`self.LineTrace for floor`))
      (if _floor_detected_
        (goto _label :!via `Reset`)
        (else
          (`/Engine/EditorBlueprintResources/StandardMacros.DoOnce` false :!label _label
            (:`Completed`
              (`/Engine/EditorBlueprintResources/StandardMacros.FlipFlop`
                (:`A`
                  (`MovementComponent.StopMovementImmediately` _charactermovement)
                  (`self.K2_AddActorWorldRotation` (struct)))
                (:`B`
                  (`MovementComponent.StopMovementImmediately` _charactermovement)
                  (`self.K2_AddActorWorldRotation` (struct)))))))))
    (:`then_1`
      (`self.Move foward `))
    (:`then_2`
      (if (not (`self.IsDead?`))
        (`self.Line Trace For Damage`)))))

(event `Move foward`
  (`self.AddMovementInput` (`self.GetActorForwardVector`)))

(event `self.damage collision.OnComponentBeginOverlap`
  (params (OverlappedComponent :type "PrimitiveComponent Object Reference") (OtherActor :type "Actor Object Reference") (OtherComp :type "PrimitiveComponent Object Reference") (OtherBodyIndex :type Integer) (bFromSweep :type Boolean) (SweepResult :type "HitResult Structure (by ref)"))
  (bind _capsulecomponent (`self.CapsuleComponent`))
  (if (`self.ActorHasTag` OtherActor "Player")
    (`PrimitiveComponent.SetSimulatePhysics` (`self.Mesh`) true)
    (`CharacterMovementComponent.DisableMovement` (`self.CharacterMovement`))
    (`PrimitiveComponent.SetCollisionResponseToChannel` _capsulecomponent "ECC_Pawn" "ECR_Ignore")
    (`PrimitiveComponent.SetCollisionResponseToChannel` _capsulecomponent "ECC_Camera" "ECR_Ignore")
    (`PrimitiveComponent.SetCollisionResponseToChannel` (`self.Mesh`) "ECC_Camera" "ECR_Ignore")
    (set `self.IsDead?` true)))

(fn `Line Trace For Damage`
  (bind _attack_damage_pos_ (`self.Attack damage pos `))
  (bind _returnvalue (`SceneComponent.K2_GetComponentLocation` _attack_damage_pos_))
  (bind (_outhit _returnvalue_2) (`KismetSystemLibrary.SphereTraceSingle` :`Start` _returnvalue :`End` (+ _returnvalue (* (`SceneComponent.K2_GetComponentRotation` _attack_damage_pos_) 150.0)) :`Radius` 20.0 :`TraceChannel` "TraceTypeQuery1" :`DrawDebugType` "ForOneFrame" :`DrawTime` 1.0))
  (if _returnvalue_2
    (`GameplayStatics.ApplyDamage` (`.HitActor` (`GameplayStatics.BreakHitResult` _outhit)) 100.0)))

(fn `line trace for wall`
  (returns (`Floor detected ` :type Boolean))
  (bind (_outhit _returnvalue) (`KismetSystemLibrary.SphereTraceSingle` (0.0 0.0 0.0) (+ (`SceneComponent.K2_GetComponentLocation` (`self.LineTrace Floor Pos`)) (* (`KismetMathLibrary.GetForwardVector` (`self.K2_GetActorRotation`)) 100.0)) 0.0 "TraceTypeQuery1"))
  (return _returnvalue))

(fn `LineTrace for floor`
  (returns (`floor detected ` :type Boolean))
  (bind _attack_damage_pos_ (`self.Attack damage pos `))
  (bind _returnvalue (`SceneComponent.K2_GetComponentLocation` _attack_damage_pos_))
  (`|ExecutionSequence`
    (:`then_0`
      (bind (_outhit _returnvalue_2) (`KismetSystemLibrary.SphereTraceSingle` :`Start` _returnvalue :`End` (+ _returnvalue (* (`SceneComponent.K2_GetComponentRotation` _attack_damage_pos_) 150.0)) :`Radius` 20.0 :`TraceChannel` "TraceTypeQuery1" :`DrawDebugType` "ForOneFrame" :`DrawTime` 1.0))
      (return (or _returnvalue_2 (stale _floor_detected_))))
    (:`then_1`
      (bind _floor_detected_ (`self.line trace for wall`)))))

(fn `UserConstructionScript`)